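; A prototype buoyancy test actor that pushes a static mesh with vertical forces at local test points.
; Trace casts a debug-drawn vertical line trace from each point.
; Hits apply force scaled by per-point mass, WaterTestHeight and the inverse of the vertical hit distance.
; Trace re-calls itself after a tiny delay, but BeginPlay is empty and nothing live starts the loop.
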(event Custom|Trace
  (bind _staticmesh (Variables|Default|GetStaticMesh))
  (bind _staticmesh_2 (Variables|Default|GetStaticMesh))
  (bind _water_test_points (Variables|Default|GetWater%20Test%20Points))
  (bind _returnvalue (Utilities|Array|Length _water_test_points))
  (bind _returnvalue_2 (Transformation|GetWorldScale _staticmesh))
  (bind _returnvalue_3 (Physics|GetMass _staticmesh_2))
  (bind (_x _y _z) (Math|Vector|BreakVector _returnvalue_2))
  (bind _returnvalue_4 (/ _returnvalue_3 _returnvalue))
  (for _array_element (Variables|Default|GetWater%20Test%20Points)
    (Variables|Default|SetTestLocation_L _array_element)
    (Variables|Default|SetForceLocation_L (Math|Transform|TransformLocation (Transformation|GetWorldTransform _staticmesh) (Variables|Default|GetTestLocation_L)))
    (bind (_outhit _returnvalue_5) (Collision|LineTraceByChannel (Variables|Default|GetForceLocation_L) (Math|Vector|MakeVector (.x (Variables|Default|GetForceLocation_L)) (.y (Variables|Default|GetForceLocation_L)) (.z (* (- (Math|Transform|TransformLocation (Transformation|GetWorldTransform _staticmesh) (Variables|Default|GetTestLocation_L)) (Math|Vector|MakeVector 0.0 0.0 (+ (/ (+ _x _y _z) 3.0) (.z (- (.Max (Components|StaticMesh|GetLocalBounds _staticmesh)) (Variables|Default|GetTestLocation_L))) (Utilities|Array|Length (Variables|Default|GetWater%20Test%20Points))))) -1.0))) "TraceTypeQuery3" false 0 "ForDuration"))
    (if _returnvalue_5
      (Class|PrimitiveComponent|AddForceatLocation (Variables|Default|GetStaticMesh) (* _returnvalue_4 (Math|Vector|MakeVector 0.0 0.0 (* (/ (Math|Vector|VectorLength _returnvalue_4) (.z (- (Variables|Default|GetForceLocation_L) (.Location (Collision|BreakHitResult _outhit))))) (Variables|Default|GetWater%20Test%20Height)))) (Variables|Default|GetForceLocation_L) "None")))
  (Utilities|FlowControl|Delay 0.001)
  (CallFunction|Trace))

(event EventBeginPlay)

(fn ConstructionScript)