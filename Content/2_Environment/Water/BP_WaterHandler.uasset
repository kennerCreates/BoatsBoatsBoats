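; BP_WaterHandler lays out the level's water surface as a square grid of static mesh tiles.
; The construction script adds MapSize squared mesh components, using integer division and modulo on the loop index for X and Y.
; Tiles are spaced by WaterSize, offset by half the map to center on the actor, and share a fixed uniform scale.
; It has no runtime logic, as BeginPlay is empty.
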(event EventBeginPlay)

(fn ConstructionScript
  (bind _mapsize (Variables|Default|GetMapSize))
  (for _index (range 0 (- (* _mapsize _mapsize) 1))
    (AddComponent|AddStaticMeshComponent false (Math|Transform|MakeTransform (Math|Vector|MakeVector (Math|Conversions|ToFloat(Integer) (* (- (/ _index (Variables|Default|GetMapSize)) (/ (Variables|Default|GetMapSize) 2)) (Variables|Default|GetWaterSize))) (Math|Conversions|ToFloat(Integer) (* (- (Math|Integer|%(Integer) _index (Variables|Default|GetMapSize)) (/ (Variables|Default|GetMapSize) 2)) (Variables|Default|GetWaterSize))) 0.0) "0, 0, 0" "5.000000,5.000000,5.000000"))))