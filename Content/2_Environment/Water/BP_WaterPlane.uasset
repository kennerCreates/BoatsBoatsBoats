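; BP_WaterPlane is a water plane actor that sizes its surface, underwater box and buoyancy plane from editable variables.
; The construction script scales WaterSurface in X and Y from EndPoint.
; UnderWaterHeight stretches Box vertically and drops it by half that height, while BuoyancyPlane's relative Z combines BuoyancyHeight with that offset, normalized by it.
; All logic is construction-time layout, as BeginPlay is empty.
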(event EventBeginPlay)

(fn ConstructionScript
  (bind _end_point (Variables|Default|GetEnd%20Point))
  (bind _returnvalue (/ _end_point 1e+02))
  (Transformation|SetWorldScale3D (Variables|Default|GetWaterSurface) (Math|Vector|MakeVector (.x _returnvalue) (.y _returnvalue) 1.0))
  (Transformation|SetRelativeScale3D (Variables|Default|GetBox) (Math|Vector|MakeVector 1.0 1.0 (/ (Variables|Default|GetUnder%20Water%20Height) 2.0)))
  (Transformation|SetRelativeLocation (Variables|Default|GetBox) (Math|Vector|MakeVector 0.0 0.0 (* (Variables|Default|GetUnder%20Water%20Height) -0.5)) false false)
  (Transformation|SetRelativeLocation (Variables|Default|GetBuoyancy%20Plane) (Math|Vector|MakeVector 0.0 0.0 (/ (+ (Variables|Default|GetBuoyancy%20Height) (* (Variables|Default|GetUnder%20Water%20Height) -0.5)) (* (Variables|Default|GetUnder%20Water%20Height) -0.5))) false false))