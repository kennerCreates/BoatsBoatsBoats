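; Procedural island generator actor that builds random terrain at BeginPlay with Geometry Script on a dynamic mesh.
; A random seed stream drives the placement and radius of tapered cones, appended with a base box.
; Solidify merges them, then smoothing, PN tessellation, two plane cuts and planar UV projection shape the final islands.
; It then releases compute meshes and nudges the actor upward; an actor spawn node is left unconnected.
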(event EventBeginPlay
  (Variables|Default|SetSeed (Math|Random|MakeRandomStream (Math|Random|RandomInteger 150)))
  (CallFunction|CreateIsland))

(fn ConstructionScript)

(fn CreateIsland
  (bind _maxspawndistance (Variables|Default|GetMaxSpawnDistance))
  (bind _seed (Variables|Default|GetSeed))
  (bind _islandsize (Variables|Default|GetIslandSize))
  (bind _maxspawndistance_2 (Variables|Default|GetMaxSpawnDistance))
  (bind _returnvalue (Math|Random|RandomUnitVectorfromStream _seed))
  (bind _returnvalue_2 (/ _maxspawndistance_2 2.0))
  (bind _returnvalue_3 (/ _maxspawndistance 1e+04))
  (bind _returnvalue_4 (* _returnvalue _returnvalue_2))
  (bind _returnvalue_5 (DynamicMeshComponent|GetDynamicMesh (Variables|DynamicMeshActor|GetDynamicMeshComponent)))
  (bind _output_get (Variables|Default|SetDyn%20Mesh _returnvalue_5))
  (DynamicMesh|Reset _output_get)
  (Utilities|Array|Clear (Variables|Default|GetSpawnPoints))
  (Utilities|FlowControl|Sequence
    (:then_0
      (for _index (range 0 (Variables|Default|GetIslands))
        (Variables|Default|SetRadius (Math|Random|RandomFloatinRangefromStream (Variables|Default|GetSeed) (.x _islandsize) (.y _islandsize)))
        (bind _returnvalue_6 (Utilities|Array|Add (Variables|Default|GetSpawnPoints) (Math|Vector|MakeVector (.x _returnvalue_4) (.y _returnvalue_4) 0.0)))
        (Class|GeometryScriptLibraryMeshPrimitiveFunctions|AppendCone :TargetMesh (Variables|Default|GetDyn%20Mesh) :Transform (Math|Transform|MakeTransform (Math|Vector|MakeVector (.x (Utilities|Array|Get(acopy) (Variables|Default|GetSpawnPoints) _returnvalue_6)) (.y (Utilities|Array|Get(acopy) (Variables|Default|GetSpawnPoints) _returnvalue_6)) -8e+02)) :BaseRadius (Variables|Default|GetRadius) :TopRadius (/ (Variables|Default|GetRadius) 4.0) :Height 1.2e+03 :RadialSteps 32 :HeightSteps 1 :Debug 0)
        (if (> (Variables|Default|GetRadius) 2e+03)
          _))
      (bind _returnvalue_7 (Class|GeometryScriptLibraryMeshPrimitiveFunctions|AppendBox :TargetMesh (Variables|Default|GetDyn%20Mesh) :Transform (Math|Transform|MakeTransform "0.000000,0.000000,-800.000000") :DimensionX _returnvalue_3 :DimensionY _returnvalue_3 :Debug 0))
      (bind _returnvalue_8 (Class|GeometryScriptLibraryMeshVoxelFunctions|ApplyMeshSolidify _returnvalue_7 (Utilities|Struct|MakeGeometryScriptSolidifyOptions (Utilities|Struct|MakeGeometryScript3DGridParameters "GridResolution" 0.25 50) 0.5 false 0.0 64) 0))
      (bind _returnvalue_9 (Class|GeometryScriptLibraryMeshNormalsFunctions|SetPerVertexNormals _returnvalue_8 0))
      (bind _returnvalue_10 (Class|GeometryScriptLibraryMeshDeformFunctions|ApplyIterativeSmoothingtoMesh :TargetMesh _returnvalue_9 :Options (Utilities|Struct|MakeGeometryScriptIterativeMeshSmoothingOptions 6 0.2 "FullMeshSelection") :Debug 0))
      (bind _returnvalue_11 (Class|GeometryScriptLibraryMeshSubdivideFunctions|ApplyPNTessellation :TargetMesh _returnvalue_10 :TessellationLevel 2 :Debug 0))
      (bind _returnvalue_12 (Class|GeometryScriptLibraryMeshBooleanFunctions|ApplyMeshPlaneCut _returnvalue_11 (Math|Transform|MakeTransform "0.000000,0.000000,-390.000000" "0.000000,0.000000,180.000000") (Utilities|Struct|MakeGeometryScriptMeshPlaneCutOptions false false false 1.0) 0))
      (bind _returnvalue_13 (Class|GeometryScriptLibraryMeshBooleanFunctions|ApplyMeshPlaneCut :TargetMesh _returnvalue_12 :CutFrame (Math|Transform|MakeTransform "0, 0, 0") :Debug 0))
      (Class|GeometryScriptLibraryMeshUVFunctions|SetMeshUVsfromPlanarProjection :TargetMesh _returnvalue_13 :PlaneTransform (Math|Transform|MakeTransform "0, 0, 0" "0, 0, 0" "100.000000,100.000000,100.000000") :Debug 0))
    (:then_1
      (DynamicMeshActor|ReleaseAllComputeMeshes)
      (Transformation|AddActorWorldOffset "0.000000,0.000000,0.050000"))))