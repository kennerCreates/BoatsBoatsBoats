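; Foliage spawner for island generation that scatters grass meshes over circular island areas once the island is finished.
; It records incoming circles, skipping any fully contained in a stored one.
; On completion, evenly distributed transforms per circle are distance-tested against already processed circles, adding one for each circle it lies outside.
; Each resulting transform becomes its own StaticMeshComponent rather than an instance.
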(event EventBeginPlay)

(event EventIslandFinished
  (CallFunction|SpawnStaticMesh(Radius) 1.2e+02 "/Game/UltraStylizedGrass/Meshes/GeometryBased/sm_grass_03.sm_grass_03" "/Game/3_Materials/Enviroment/M_Grass.M_Grass" "(X=0.500000,Y=1.000000)" false "NoCollision"))

(event EventAddIslandData
  (params (CircleLocation :type Vector :default "0, 0, 0") (CircleRadius :type Float%20%28double-precision%29))
  (Variables|Default|SetAddNewIsland true)
  (CallFunction|CheckNewIslandLocation CircleLocation CircleRadius))

(fn ConstructionScript)

(fn CheckNewIslandLocation
  (params (Location :type Vector) (Radius :type Float%20%28double-precision%29))
  (bind _keys (Utilities|Map|Keys (Variables|Default|GetIslandCircles)))
  (for _array_element _keys
    (if (> (.Value (Utilities|Map|Find (Variables|Default|GetIslandCircles) _array_element)) (+ (Math|Vector|Distance(Vector) _array_element Location) Radius))
      (Variables|Default|SetAddNewIsland false)))
  (if (Variables|Default|GetAddNewIsland)
    (Utilities|Map|Add (Variables|Default|GetIslandCircles) Location Radius)))

(fn CheckTransformLocations
  (params (Transforms :type Array%20of%20Transforms) (Size%20SM :type Float%20%28double-precision%29))
  (bind _islandcircles_checked (Variables|Default|GetIslandCircles_Checked))
  (for _array_element Transforms
    (LocalVariables|SetTransformToCheck _array_element)
    (if (> (Utilities|Map|Length (Variables|Default|GetIslandCircles_Checked)) 0)
      (bind _keys (Utilities|Map|Keys _islandcircles_checked))
      (for _array_element_2 _keys
        (if (>= (Math|Vector|Distance(Vector) (.Location (Math|Transform|BreakTransform (LocalVariables|GetTransformToCheck))) _array_element_2) (- (.Value (Utilities|Map|Find _islandcircles_checked _array_element_2)) (/ Size%20SM 3.0)))
          (Utilities|Array|Add (Variables|Default|GetTransforms%20to%20Spawn) (LocalVariables|GetTransformToCheck))))
      (else
        (Utilities|Array|Add (Variables|Default|GetTransforms%20to%20Spawn) (LocalVariables|GetTransformToCheck))))))

(fn SpawnStaticMesh(Radius)
  (params (Size_SM :type Float%20%28double-precision%29) (Static%20Mesh :type Static%20Mesh%20Object%20Reference) (Material :type Material%20Interface%20Object%20Reference) (Scale :type Vector%202D%20Structure) (CastShadow :type Boolean) (Collision :type ECollisionEnabled%20Enum :default "NoCollision"))
  (Utilities|Array|Clear (Variables|Default|GetTransforms%20to%20Spawn))
  (Utilities|Map|Clear (Variables|Default|GetIslandCircles_Checked))
  (bind _keys (Utilities|Map|Keys (Variables|Default|GetIslandCircles)))
  (for _array_element _keys
    (bind _transformstospawn (CallFunction|TransformsEvenRadius _array_element (.Value (Utilities|Map|Find (Variables|Default|GetIslandCircles) _array_element)) Size_SM Scale))
    (CallFunction|CheckTransformLocations _transformstospawn Size_SM)
    (Utilities|Map|Add (Variables|Default|GetIslandCircles_Checked) _array_element (.Value (Utilities|Map|Find (Variables|Default|GetIslandCircles) _array_element))))
  (for _array_element_2 (Variables|Default|GetTransforms%20to%20Spawn)
    (bind _returnvalue (AddComponent|AddStaticMeshComponent false _array_element_2))
    (Components|StaticMesh|SetStaticMesh _returnvalue Static%20Mesh)
    (Rendering|Material|SetMaterial _returnvalue 0 Material)
    (Rendering|SetCastShadow _returnvalue CastShadow)
    (Collision|SetCollisionEnabled _returnvalue Collision)))

(fn IslandSeed
  (return ""))